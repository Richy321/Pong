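; Pong HUD that owns the in-match scoreboard and starting countdown and shows the end-of-game result.
; BeginPlay adds scoreboard, countdown and game-finished widgets to the viewport, the latter two hidden.
; Custom events forward score and countdown values and toggle widget visibility.
; Game start and finish switch screens through MenuManager; the result goes to its EndGameMenu widget, leaving the locally created finished widget unused.
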(event EventBeginPlay
  (bind _playerowner (Variables|Default|GetPlayerOwner))
  ;[1 1 1] Create Game Finished Popup
  (bind _returnvalue (UserInterface|CreateWidget "/Game/UI/W_GameFinishedWidget.W_GameFinishedWidget_C" _playerowner))
  (bind _output_get (Variables|Default|SetGameFinishedWidget _returnvalue))
  (UserInterface|Viewport|AddtoViewport _output_get 0)
  (Widget|SetVisibility _output_get "Hidden")
  ;[1 1 1] Create scoreboard
  (bind _returnvalue_2 (UserInterface|CreateWidget "/Game/UI/W_ScoreBoardWidget.W_ScoreBoardWidget_C" _playerowner))
  (UserInterface|Viewport|AddtoViewport _returnvalue_2 0)
  (Variables|Default|SetScoreboardWidget _returnvalue_2)
  ;[1 1 1] Create Countdown widget
  (bind _returnvalue_3 (UserInterface|CreateWidget "/Game/UI/W_StartingCountdownWidget.W_StartingCountdownWidget_C" _playerowner))
  (UserInterface|Viewport|AddtoViewport _returnvalue_3 0)
  (bind _output_get_2 (Variables|Default|SetStartCountdownWidget _returnvalue_3))
  (Widget|SetVisibility _output_get_2 "Hidden"))

(event Collision|EventActorBeginOverlap
  (params (OtherActor :type Actor%20Object%20Reference)))

(event EventSetScore
  (params (Score :type Game%20Score%20Structure%20%28by%20ref%29))
  ;[1 1 1] Set Score
  (Default|SetScore (Variables|Default|GetScoreboardWidget) Score))

(event EventShowGameFinishedUI
  (params (Result :type Game%20Score%20Structure))
  ;[1 1 1] Show Game Finished UI
  (bind _returnvalue (Class|MenuManager|GetScreenWidget (Variables|Default|GetMenuManager) "EndGameMenu"))
  (bind _asw_game_finished_widget (Utilities|Casting|CastToW_GameFinishedWidget _returnvalue))
  (Default|SetScore _asw_game_finished_widget Result)
  (Class|MenuManager|GotoScreen (Variables|Default|GetMenuManager) "EndGameMenu"))

(event EventUpdateStartingCountdown
  (params (CountdownTime :type Float%20%28single-precision%29))
  ;[1 1 1] Update Starting Countdown
  (Default|SetCountdownValue (Variables|Default|GetStartCountdownWidget) CountdownTime))

(event EventShowGameStartingUI
  ;[1 1 1] Game Starting
  (Class|MenuManager|GotoScreen (Variables|Default|GetMenuManager) "None")
  (Default|Show (Variables|Default|GetStartCountdownWidget)))

(event EventTick
  (params (DeltaSeconds :type Float%20%28single-precision%29)))

(event EventShowGameUI
  (bind _startcountdownwidget (Variables|Default|GetStartCountdownWidget))
  ;[1 1 1] Show Game UI
  (Widget|SetVisibility (Variables|Default|GetScoreboardWidget) "Visible")
  (if (Utilities|Enum|Equal(Enum) (Widget|GetVisibility _startcountdownwidget) "Visible")
    (Default|Hide _startcountdownwidget)))

(event EventHideGameUI
  ;[1 1 1] Hide Game UI
  (Widget|SetVisibility (Variables|Default|GetScoreboardWidget) "Hidden"))

(fn ConstructionScript)